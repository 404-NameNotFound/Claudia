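; 2D lift that shuttles a sprite between its origin and EndLocation on a timeline scaled to TravelTimeInSeconds.
; Each finished run waits StopDelay, then LiftForward or LiftBackward sends it the other way.
; A safety collider flips the active timeline's direction when Claudia_Blueprint overlaps it.
; The construction script applies LiftColor and uses TestEndLocation to place the sprite at either endpoint.
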(event OnComponentBeginOverlap(SafteyCollider)
  (params (OtherActor :type Actor%20Object%20Reference) (OtherComp :type Primitive%20Component%20Object%20Reference) (OtherBodyIndex :type Integer) (bFromSweep :type Boolean) (SweepResult :type Hit%20Result%20Structure%20%28by%20ref%29))
  (bind _lift_timeline (Variables|Default|GetLift%20Timeline))
  ;[1 1 1] Player Detection Logic
  (Utilities|Casting|CastToClaudia_Blueprint OtherActor)
  (if (Components|Activation|IsActive _lift_timeline)
    (if (Class|TimelineComponent|IsReversing _lift_timeline)
      (bind (_direction _lerp_alpha) (Timeline|Lift%20Timeline Play)
        (:Update
          (Transformation|SetRelativeLocation (Variables|Default|GetLiftSprite) (Math|Vector|Lerp(Vector) "0, 0, 0" (Variables|LiftControls|GetEndLocation) _lerp_alpha) false))
        (:Finished
          (Utilities|FlowControl|Delay (Variables|LiftControls|GetStopDelay))
          (switch Utilities|FlowControl|Switch|SwitchonETimelineDirection _direction
            (:Forward
              (CallFunction|LiftBackward))
            (:Backward
              (CallFunction|LiftForward)))))
      (else
        (Timeline|Lift%20Timeline Reverse)))))

(event Custom|LiftForward
  (bind (_direction _lerp_alpha) (Timeline|Lift%20Timeline PlayFromStart)
    (:Update
      (Transformation|SetRelativeLocation (Variables|Default|GetLiftSprite) (Math|Vector|Lerp(Vector) "0, 0, 0" (Variables|LiftControls|GetEndLocation) _lerp_alpha) false))
    (:Finished
      (Utilities|FlowControl|Delay (Variables|LiftControls|GetStopDelay))
      (switch Utilities|FlowControl|Switch|SwitchonETimelineDirection _direction
        (:Forward
          (CallFunction|LiftBackward))
        (:Backward
          (CallFunction|LiftForward))))))

(event Custom|LiftBackward
  (bind (_direction _lerp_alpha) (Timeline|Lift%20Timeline ReverseFromEnd)
    (:Update
      (Transformation|SetRelativeLocation (Variables|Default|GetLiftSprite) (Math|Vector|Lerp(Vector) "0, 0, 0" (Variables|LiftControls|GetEndLocation) _lerp_alpha) false))
    (:Finished
      (Utilities|FlowControl|Delay (Variables|LiftControls|GetStopDelay))
      (switch Utilities|FlowControl|Switch|SwitchonETimelineDirection _direction
        (:Forward
          (CallFunction|LiftBackward))
        (:Backward
          (CallFunction|LiftForward))))))

(event EventBeginPlay
  (Components|Timeline|SetPlayRate (Variables|Default|GetLift%20Timeline) (/ 1.0 (Variables|LiftControls|GetTravelTimeInSeconds)))
  (Variables|LiftControls|SetTestEndLocation true))

(fn ConstructionScript
  (bind _liftsprite (Variables|Default|GetLiftSprite))
  (Transformation|SetRelativeLocation _liftsprite (Math|Vector|SelectVector (Variables|LiftControls|GetEndLocation) "0, 0, 0" (Variables|LiftControls|GetTestEndLocation)) false)
  (Sprite|SetSpriteColor _liftsprite (Variables|LiftControls|GetLiftColor)))