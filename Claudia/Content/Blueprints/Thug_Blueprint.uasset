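; Thug_Blueprint is a 2D enemy thug that reacts to the player character's proximity and damages it on contact.
; Each tick it measures distance to the player, switching its flipbook between idle and pipe-hit at DetectPlayerDistance and mirroring the sprite's X scale to face the player.
; Capsule hits against Claudia_Blueprint actors apply damage directly, independent of the attack animation.
; Debug prints remain throughout.
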(event OnComponentHit(CapsuleComponent)
  (params (OtherActor :type Actor%20Object%20Reference) (OtherComp :type Primitive%20Component%20Object%20Reference) (NormalImpulse :type Vector :default "0, 0, 0") (Hit :type Hit%20Result%20Structure%20%28by%20ref%29))
  ;[1 1 1] Hit shit
  (Variables|Default|SetHitEnemy OtherActor)
  (if (Utilities|ClassIsChildOf (Utilities|GetClass (Variables|Default|GetHitEnemy)) "/Game/Blueprints/Claudia_Blueprint.Claudia_Blueprint_C")
    (Game|Damage|ApplyDamage (Variables|Default|GetHitEnemy) 1.0 0 0)))

(event EventTick
  (params (DeltaSeconds :type Float%20%28single-precision%29))
  (bind _thugsprite (Variables|Default|GetthugSprite))
  ;[1 1 1] Get Player Avatar
  (bind _ascharacter (Utilities|Casting|CastToCharacter (Game|Player|GetPlayerPawn 0))
    (:then
      ;[1 1 1] Testing Purposes Only.
      (Development|PrintString (Utilities|String|ToString(Float) (Math|Vector|VectorLength (- (Transformation|GetActorLocation) (Transformation|GetActorLocation _ascharacter)))))
      (if (>= (Math|Vector|VectorLength (- (Transformation|GetActorLocation) (Transformation|GetActorLocation _ascharacter))) (Variables|Default|GetDetectPlayerDistance))
        (Sprite|SetFlipbook (Variables|Default|GetthugSprite) (Variables|Default|GetThugIdle))
        (Development|PrintString "Nobody there lol")
        (else
          (Sprite|SetFlipbook (Variables|Default|GetthugSprite) (Variables|Default|GetThugPipeHit))
          (Development|PrintString "Hello")))
      (if (>= (.X (Math|Vector|BreakVector (Transformation|GetActorLocation (Game|Player|GetPlayerPawn 0)))) (.X (Math|Vector|BreakVector (Transformation|GetActorLocation))))
        (Transformation|SetWorldScale3D _thugsprite "1.700000,1.000000,1.700000")
        (else
          (Transformation|SetWorldScale3D _thugsprite "-1.700000,1.000000,1.700000"))))
    (:CastFailed
      (Development|PrintString "Failed"))))

(fn ConstructionScript)