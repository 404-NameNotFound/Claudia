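; Bullet actor that plays a grapple-shoot sound on spawn and destroys itself when its lifetime runs out.
; BeginPlay marks the bullet alive and plays the sound at the world origin, not at the actor's location.
; Tick subtracts delta time from the remaining life, then resets it and destroys the actor once it reaches zero.
; The graphs contain no movement or hit logic.
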(event EventBeginPlay
  (Variables|Default|SetbulletIsAlive true)
  (if (Variables|Default|GetbulletIsAlive)
    (Audio|PlaySoundatLocation "/Game/Sounds/ClaudiaSounds/GrappleShoot.GrappleShoot" "0, 0, 0")))

(event EventTick
  (params (DeltaSeconds :type Float%20%28single-precision%29))
  (Variables|Default|SetdeltSeconds DeltaSeconds)
  (if (Variables|Default|GetbulletIsAlive)
    (Variables|Default|SetbulletLife (- (Variables|Default|GetbulletLife) (Variables|Default|GetdeltSeconds)))
    (if (<= (Variables|Default|GetbulletLife) 0.0)
      (Variables|Default|SetbulletLife 4.0)
      (Actor|DestroyActor))))

(fn ConstructionScript)