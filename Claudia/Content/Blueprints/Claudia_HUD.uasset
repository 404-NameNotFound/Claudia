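; Claudia_HUD is a HUD Blueprint that draws momentum and health textures and a custom crosshair cursor.
; Each DrawHUD call draws both textures at quarter scale, with momentum below health, as static images with no bound values.
; The crosshair follows player 0's mouse position, corrected by half the difference between canvas and viewport size and shifted up-left by a fixed offset.
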(event EventDrawHUD
  (params (SizeX :type Integer) (SizeY :type Integer))
  (bind _returnvalue (Game|GetPlayerController 0))
  (bind _returnvalue_2 (Math|Float|MakeLiteralFloat 32.0))
  (bind (_sizex _sizey) (HUD|GetViewportSize _returnvalue))
  (bind _returnvalue_3 (/ _returnvalue_2 2.0))
  (bind (_locationx _locationy) (Game|Player|GetMousePosition _returnvalue))
  (Class|HUD|DrawTextureSimple "/Game/HUD/HUD_Momentum_Texture.HUD_Momentum_Texture" 0.0 1e+02 0.25 false)
  (Class|HUD|DrawTextureSimple "/Game/HUD/HUD_Health_Texture.HUD_Health_Texture" 0.0 0.0 0.25 false)
  ;[1 1 1] Draw Cursor
  (Canvas|DrawTexture "/Game/Textures/crosshair.crosshair" (- (+ (/ (Math|Conversions|ToFloat(Integer) (- SizeX _sizex)) 2.0) _locationx) _returnvalue_3) (- (+ _locationy (/ (Math|Conversions|ToFloat(Integer) (- SizeY _sizey)) 2.0)) _returnvalue_3) _returnvalue_3 _returnvalue_3 0.0 0.0 1.0 1.0 "(R=1.000000,G=1.000000,B=1.000000,A=1.000000)"))

(fn ConstructionScript)