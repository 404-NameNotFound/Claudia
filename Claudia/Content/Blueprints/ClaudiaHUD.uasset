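; ClaudiaHUD is a HUD Blueprint that draws a custom material-based mouse cursor on screen.
; On each DrawHUD event, it reads player 0's mouse position and draws the LevelPrototype material there as a small square.
; It adds half the difference between HUD canvas and viewport size to the position, then shifts by the square's full drawn size, placing its bottom-right corner at that point.
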(event EventDrawHUD
  (params (SizeX :type Integer) (SizeY :type Integer))
  (bind _returnvalue (Game|GetPlayerController 0))
  (bind _returnvalue_2 (Math|Float|MakeLiteralFloat 32.0))
  (bind (_locationx _locationy) (Game|Player|GetMousePosition _returnvalue))
  (bind (_sizex _sizey) (HUD|GetViewportSize _returnvalue))
  (bind _returnvalue_3 (/ _returnvalue_2 2.0))
  ;[1 1 1] Draw Custom Cursor
  (Canvas|DrawMaterial "/Game/Materials/LevelPrototype.LevelPrototype" (- (+ (/ (Math|Conversions|ToFloat(Integer) (- SizeX _sizex)) 2.0) _locationx) _returnvalue_3) (- (+ (/ (Math|Conversions|ToFloat(Integer) (- SizeY _sizey)) 2.0) _locationy) _returnvalue_3) _returnvalue_3 _returnvalue_3 0.0 0.0 1.0 1.0))

(fn ConstructionScript)